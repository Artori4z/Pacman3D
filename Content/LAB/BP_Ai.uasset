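; BP_Ai is an NPC character the player can talk to.
; Its Box overlap flags the player's AiOverlap, and leaving restores the random walk speed and resets dialogue state.
; Talk halts movement and writes a line chosen by DialogueLine into AiDialogue widgets, though its clearing branch is unreachable.
; The random-point wander loop is disconnected, and the EnergyCheck macro is an unfinished stub.
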(event `self.ReceiveBeginPlay`
  (bind _output_get (set `self.WalkSpeed` (`KismetMathLibrary.RandomFloatInRange` 100.0 450.0))))

(event `self.box.OnComponentBeginOverlap`
  (params (OverlappedComponent :type "PrimitiveComponent Object Reference") (OtherActor :type "Actor Object Reference") (OtherComp :type "PrimitiveComponent Object Reference") (OtherBodyIndex :type Integer) (bFromSweep :type Boolean) (SweepResult :type "HitResult Structure (by ref)"))
  (bind _asbp_third_person_character (cast `/Game/ThirdPerson/Blueprints/BP_ThirdPersonCharacter` OtherActor))
  (set `/Game/ThirdPerson/Blueprints/BP_ThirdPersonCharacter.AiOverlap` true _asbp_third_person_character)
  (`KismetSystemLibrary.PrintString` "BRRR"))

(event `self.box.OnComponentEndOverlap`
  (params (OverlappedComponent :type "PrimitiveComponent Object Reference") (OtherActor :type "Actor Object Reference") (OtherComp :type "PrimitiveComponent Object Reference") (OtherBodyIndex :type Integer))
  (bind _asbp_third_person_character (cast `/Game/ThirdPerson/Blueprints/BP_ThirdPersonCharacter` OtherActor))
  (set `/Game/ThirdPerson/Blueprints/BP_ThirdPersonCharacter.AiOverlap` false _asbp_third_person_character)
  (`KismetSystemLibrary.PrintString` "BURRRRRH")
  (set `self.IsTalking` false)
  (set `CharacterMovementComponent.MaxWalkSpeed` (`self.WalkSpeed`) (`self.CharacterMovement`))
  (`Widget.SetVisibility` (stale `Talk` _array_element) "Visible")
  (set `self.DialogueLine` 0))

(event `Talk`
  (bind _dialogueline (`self.DialogueLine`))
  (set `CharacterMovementComponent.MaxWalkSpeed` 0.0 (`self.CharacterMovement`))
  (`KismetSystemLibrary.PrintString` "I going to eat you")
  (bind _foundwidgets (`WidgetBlueprintLibrary.GetAllWidgetsOfClass` "/Game/LAB/AiDialogue.AiDialogue_C"))
  (for _array_element _foundwidgets
    (if (== _dialogueline 1)
      (set `/Game/LAB/AiDialogue.Dialogue` (`self.Dialogue`) _array_element)
      (`Widget.SetVisibility` _array_element "Visible")
      (elif (>= _dialogueline 2)
        (set `/Game/LAB/AiDialogue.Dialogue` (`self.Dialogue2`) _array_element)
        (`Widget.SetVisibility` _array_element "Visible")
        (elif (>= _dialogueline 3)
          (set `self.DialogueLine` 0)
          (set `/Game/LAB/AiDialogue.Dialogue` "" _array_element))))))

(fn `UserConstructionScript`)